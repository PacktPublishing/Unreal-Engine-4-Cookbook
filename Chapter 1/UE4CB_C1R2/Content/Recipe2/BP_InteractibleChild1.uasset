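; Child interactible Blueprint in a Recipe2 folder that gives its own response to an interface event.
; On that event it destroys the current Mesh if valid, adds a new static mesh component as Mesh, and sets it to a rock.
; It then prints its display name in green to the screen to confirm the call.
; The construction script only calls the parent, and the default event nodes are disabled.
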(event `/Game/Recipe2/BPI_Interactible.InterfaceEvent`
  (bind _mesh (`self.Mesh`))
  ;[1 1 1] Custom Functionality
  (`/Engine/EditorBlueprintResources/StandardMacros.IsValid` _mesh
    (:`Is Valid`
      (`ActorComponent.K2_DestroyComponent` _mesh))
    (:`Is Not Valid`
      _))
  (bind _returnvalue (`AddComponent|NODE_AddStaticMeshComponent-0`))
  (bind _output_get (set `self.Mesh` _returnvalue))
  (`StaticMeshComponent.SetStaticMesh` _output_get "/Game/StarterContent/Props/SM_Rock.SM_Rock")
  (`KismetSystemLibrary.PrintString` (`KismetStringLibrary.Concat_StrStr` (`KismetSystemLibrary.GetDisplayName` self) " Interface Event Called") true false (struct :`G` 1.0 :`B` 0.061501 :`A` 1.0)))

(fn `UserConstructionScript`
  (`parent.UserConstructionScript`))