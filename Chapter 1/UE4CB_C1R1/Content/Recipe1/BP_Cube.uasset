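; BP_Cube is an actor that changes its mesh colour in response to an event dispatcher on the player's ThirdPersonCharacter.
; On BeginPlay it creates a dynamic M_Cube material instance and binds ChangeCubeColour to the character's UpdateCubeColour dispatcher.
; When the dispatcher fires, SetCubeColour validates the instance and writes the received colour to its Colour vector parameter.
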(event `self.ReceiveBeginPlay`
  ;[1 1 1] Create Material Instance
  (bind _returnvalue (`PrimitiveComponent.CreateDynamicMaterialInstance` (`self.StaticMesh`) 0 "/Game/Recipe1/M_Cube.M_Cube" "None"))
  (set `self.MID_Cube` _returnvalue)
  ;[1 1 1] Recipe 1 Code - Bind Dispatcher to Event on Begin Play
  (bind _asthird_person_character (cast `/Game/ThirdPersonBP/Blueprints/ThirdPersonCharacter` (`GameplayStatics.GetPlayerCharacter` 0)))
  (add `/Game/ThirdPersonBP/Blueprints/ThirdPersonCharacter.UpdateCubeColour` _asthird_person_character (delegate `ChangeCubeColour`)))

(event `ChangeCubeColour`
  (params (Colour :type "LinearColor Structure"))
  ;[1 1 1] Recipe 1 Code - Bind Dispatcher to Event on Begin Play
  (`self.SetCubeColour` Colour))

(fn `SetCubeColour`
  (params (NewColour :type "LinearColor Structure"))
  (bind _mid_cube (`self.MID_Cube`))
  (`/Engine/EditorBlueprintResources/StandardMacros.IsValid` _mid_cube
    (:`Is Valid`
      (`MaterialInstanceDynamic.SetVectorParameterValue` _mid_cube "Colour" NewColour))))

(fn `UserConstructionScript`)