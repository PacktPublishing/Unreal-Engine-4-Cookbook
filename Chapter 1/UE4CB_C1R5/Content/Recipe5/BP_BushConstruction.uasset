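; BP_BushConstruction is an actor that scatters bush meshes over the ground around itself from its construction script.
; For each of NumberOfActors, it picks a random XY offset within a square around the actor and line-traces along negative up against WorldStatic objects.
; Each hit adds an SM_Bush static mesh component at ground height, with random yaw and per-axis scale.
; Randomness is unseeded, and the event graph is empty.
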(fn `UserConstructionScript`
  (bind _returnvalue (`KismetMathLibrary.RandomFloatInRange` 0.6 1.1))
  (bind _randomlocation (`self.RandomLocation`))
  (for _ (range 1 (+ (`self.NumberOfActors`) 1))
    (set `self.RandomLocation` (`KismetMathLibrary.MakeVector` (+ (`KismetMathLibrary.RandomFloatInRange` -300.0 300.0) (.x (`self.K2_GetActorLocation`))) (+ (`KismetMathLibrary.RandomFloatInRange` -300.0 300.0) (.y (`self.K2_GetActorLocation`))) (.z (`self.K2_GetActorLocation`))))
    (bind (_outhit _returnvalue_2) (`KismetSystemLibrary.LineTraceSingleForObjects` :`Start` _randomlocation :`End` (+ _randomlocation (* (`KismetMathLibrary.GetUpVector` (`self.K2_GetActorRotation`)) (* (`self.TraceDistance`) -1.0))) :`ObjectTypes` (`|MakeArray` "ObjectTypeQuery1" :!type "EObjectTypeQuery Enum") :`bTraceComplex` true :`DrawTime` 0.5))
    (if _returnvalue_2
      (bind _returnvalue_3 (`AddComponent|NODE_AddStaticMeshComponent-1` :`bManualAttachment` true :`RelativeTransform` (`KismetMathLibrary.MakeTransform` (`KismetMathLibrary.MakeVector` (.x (`self.RandomLocation`)) (.y (`self.RandomLocation`)) (.z (`.ImpactPoint` (`GameplayStatics.BreakHitResult` _outhit)))) (`KismetMathLibrary.MakeRotator` 0.0 0.0 (`KismetMathLibrary.RandomFloatInRange` 0.0 360.0)) (`KismetMathLibrary.MakeVector` _returnvalue _returnvalue _returnvalue))))
      (`self.K2_AttachToComponent` _returnvalue_3 "None" "KeepRelative" "KeepRelative" "KeepRelative")
      (`StaticMeshComponent.SetStaticMesh` _returnvalue_3 "/Game/StarterContent/Props/SM_Bush.SM_Bush"))))